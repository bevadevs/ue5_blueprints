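; BP_CubitoPadre is a parent actor from an inheritance exercise that spawns with a random look and destroys itself after a short random lifetime.
; Its construction script randomly picks a cylinder or chamfered cube mesh and applies a dynamic instance of M_ColorVariable with a random color parameter, re-rolling whenever the script reruns.
; BeginPlay waits a random delay before destroying the actor; the TiempoDeVida variable is unused.
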(event EventBeginPlay
  (Utilities|FlowControl|Delay (Math|Random|RandomFloatinRange 1.0 6.0))
  (Actor|DestroyActor))

(fn ConstructionScript
  ;[1 1 1] Se lanza cada vez que el objeto se compila y/o modificas alguno de sus valores.
  (Components|StaticMesh|SetStaticMesh (Variables|Default|GetCube) (select (Math|Random|RandomBool) "/Game/LevelPrototyping/Meshes/SM_Cylinder.SM_Cylinder" "/Game/LevelPrototyping/Meshes/SM_ChamferCube.SM_ChamferCube"))
  (bind _returnvalue (Rendering|Material|CreateDynamicMaterialInstance "/Game/Materials/M_ColorVariable.M_ColorVariable" "None" "None" :!class /Script/Engine.KismetMaterialLibrary))
  (bind _output_get (Variables|Default|SetInstanciaMaterialColores _returnvalue))
  (Rendering|Material|SetVectorParameterValue _output_get "ParametroColor" (Utilities|Struct|MakeLinearColor (Math|Random|RandomFloat) (Math|Random|RandomFloat) (Math|Random|RandomFloat) (Math|Random|RandomFloat)) :!class /Script/Engine.MaterialInstanceDynamic)
  (Rendering|Material|SetMaterial (Variables|Default|GetCube) 0 _output_get))