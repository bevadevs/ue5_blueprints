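; BP_CoinSpawner is an actor that scatters BP_Monedita coins around its location when play begins.
; It makes fifty attempts at random XY points within CoinSpawnArea, tracing vertically on the Visibility channel to find the surface height.
; It spawns a coin at the hit height unless the trace hit another coin, so coins avoid stacking and the total can fall below fifty.
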(event EventBeginPlay
  (bind _returnvalue (Transformation|GetActorLocation))
  (bind _coinspawnarea (Variables|Default|GetCoinSpawnArea))
  (bind (_x _y) (Math|Vector|BreakVector _returnvalue))
  (bind _returnvalue_2 (* -1.0 _coinspawnarea))
  (for _index (range 0 49)
    (bind _output_get (Variables|Default|SetCoinX (+ _x (Math|Random|RandomFloatinRange _returnvalue_2 _coinspawnarea))))
    (bind _output_get_2 (Variables|Default|SetCoinY (+ _y (Math|Random|RandomFloatinRange _returnvalue_2 _coinspawnarea))))
    (bind _outhit (Collision|LineTraceByChannel (Math|Vector|MakeVector _output_get _output_get_2 2e+03) (Math|Vector|MakeVector _output_get _output_get_2 -2e+03) "TraceTypeQuery1" false 0 "ForOneFrame"))
    (if (not (== (Utilities|GetClass (.HitActor (Collision|BreakHitResult _outhit))) "/Game/Blueprints/BP_Monedita.BP_Monedita_C"))
      (Game|SpawnActorfromClass "/Game/Blueprints/BP_Monedita.BP_Monedita_C" (Math|Transform|MakeTransform (Math|Vector|MakeVector (Variables|Default|GetCoinX) (Variables|Default|GetCoinY) (.Z (Math|Vector|BreakVector (.Location (Collision|BreakHitResult _outhit))))) "0, 0, 0" "1.000000,1.000000,1.000000") "Undefined" "MultiplyWithRoot" 0 0))))

(fn ConstructionScript)