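; Security camera actor that smoothly turns to track the first player character.
; Each Tick, it computes a look-at rotation toward the player, clamps only the yaw to an angular range, and keeps pitch and roll unrestricted.
; It eases a stored CurrentRotation toward that target with RInterpTo, applying the result to the whole actor and saving it back for the next frame.
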(event EventBeginPlay)

(event Collision|EventActorBeginOverlap
  (params (OtherActor :type Actor%20Object%20Reference)))

(event EventTick
  (params (DeltaSeconds :type Float%20%28single-precision%29))
  (bind _returnvalue (Game|GetPlayerCharacter 0))
  (bind _returnvalue_2 (Transformation|GetActorLocation))
  (bind _returnvalue_3 (Transformation|GetActorLocation _returnvalue))
  (bind _returnvalue_4 (Math|Rotator|FindLookatRotation _returnvalue_2 _returnvalue_3))
  (bind (_roll _pitch _yaw) (Math|Rotator|BreakRotator _returnvalue_4))
  (Transformation|SetActorRotation (Math|Interpolation|RInterpTo (Variables|Default|GetCurrentRotation) (Math|Rotator|MakeRotator _roll _pitch (Math|Float|ClampAngle _yaw 15.0 -1.9e+02)) DeltaSeconds 5.0))
  (Variables|Default|SetCurrentRotation (Math|Interpolation|RInterpTo (Variables|Default|GetCurrentRotation) (Math|Rotator|MakeRotator _roll _pitch (Math|Float|ClampAngle _yaw 15.0 -1.9e+02)) DeltaSeconds 5.0)))

(fn ConstructionScript)