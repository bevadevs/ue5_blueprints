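; Practice moving-platform Blueprint that uses an InterpToMovement component to travel between point A and point B.
; On BeginPlay it takes the actor's location as A, offsets it along world X for B, and assigns both as absolute control points.
; It sets a Duration variable without passing it to the component.
; Disconnected leftovers include a relative-point setup with configurable duration and a construction-script copy with a shorter offset.
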(event EventBeginPlay
  (Variables|Default|SetDuration 5.0)
  (bind _output_get (Variables|Default|SetAPoint (Transformation|GetActorLocation)))
  (bind _output_get_2 (Variables|Default|SetBPoint (+ _output_get "100.000000,0.000000,0.000000")))
  (Variables|/Script/Engine.InterpToMovementComponent|SetControlPoints (Variables|Default|GetInterpToMovement) (Utilities|Array|MakeArray (Utilities|Struct|MakeInterpControlPoint _output_get false) (Utilities|Struct|MakeInterpControlPoint _output_get_2 false))))

(fn ConstructionScript)