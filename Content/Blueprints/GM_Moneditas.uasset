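; GM_Moneditas is a game mode Blueprint running a countdown and a score for what appears to be a coin game.
; A looping one-second timer counts down and prints the remaining time, then prints GAME OVER and quits after a delay.
; SumarPuntos adds and prints points, then fires a forward debug line trace whose result is unused.
; Stage advancement, which would reset the time from EtapasInfo keys, is unconnected.
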(event Custom|SumarPuntos
  (params (Puntuacion%20A%20Sumar :type Integer))
  (bind _output_get (Variables|Default|SetPuntuacionTotal (+ Puntuacion%20A%20Sumar (Variables|Default|GetPuntuacionTotal))))
  (Development|PrintString (Utilities|String|ToString(Integer) _output_get))
  (Collision|LineTraceByChannel (Transformation|GetActorLocation) (+ (* (Transformation|GetActorForwardVector) (Variables|Default|GetDistanciaHaciaDelante)) (Transformation|GetActorLocation)) "TraceTypeQuery1" false 0 "ForOneFrame"))

(event Custom|CuentaAtras
  ;[1 1 1] Timer
  (bind _result (Math|Integer|DecrementInt (Variables|Default|GetTiempoRestante))
    (:%20%20
      (if (>= _result 0)
        (Development|PrintString (Utilities|String|Append "Tiempo restante:" (Utilities|String|ToString(Integer) _result)))
        (else
          (Development|PrintString "GAME OVER")
          (Utilities|FlowControl|Delay 2.0)
          (Game|QuitGame 0 "Quit" false))))))

(event EventBeginPlay
  ;[1 1 1] Timer
  (Variables|Default|SetTiempoRestante (Variables|Default|GetTiempoDeJuego))
  (bind _returnvalue (Utilities|Time|SetTimerbyEvent (delegate Custom|CuentaAtras) 1.0 true))
  (Variables|Default|SetTimer%20Handler _returnvalue))

(fn ConstructionScript)