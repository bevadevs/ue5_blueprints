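; Coin pickup that awards points to the third-person character and destroys itself when touched.
; The construction script randomly picks bronze, silver or gold, setting the cylinder's material and matching coin value, so the type rerolls whenever construction reruns.
; Box overlap checks for the exact BP_ThirdPersonCharacter class, calls DestroyActor, then passes the value to the character's SumarPuntos.
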(event OnComponentBeginOverlap(Box)
  (params (OverlappedComponent :type Primitive%20Component%20Object%20Reference) (OtherActor :type Actor%20Object%20Reference) (OtherComp :type Primitive%20Component%20Object%20Reference) (OtherBodyIndex :type Integer) (bFromSweep :type Boolean) (SweepResult :type Hit%20Result%20Structure%20%28by%20ref%29))
  (if (== (Utilities|GetClass OtherActor) "/Game/ThirdPerson/Blueprints/BP_ThirdPersonCharacter.BP_ThirdPersonCharacter_C")
    (Actor|DestroyActor)
    (bind _asbp_third_person_character (Utilities|Casting|CastToBP_ThirdPersonCharacter OtherActor))
    (Default|SumarPuntos _asbp_third_person_character (Variables|Default|GetCoinValue))))

(event EventBeginPlay)

(event Collision|EventActorBeginOverlap
  (params (OtherActor :type Actor%20Object%20Reference)))

(event EventTick
  (params (DeltaSeconds :type Float%20%28single-precision%29)))

(fn ConstructionScript
  (bind _output_get (LocalVariables|SetTypeOfCoin (Math|Random|RandomIntegerinRange 0 2)))
  (Rendering|Material|SetMaterial (Variables|Default|GetCylinder) 0 (Utilities|Select :Index _output_get :Option%200 "/Game/Materials/M_Bronce.M_Bronce" :Option%201 "/Game/Materials/M_Silver.M_Silver" :Option%202 "/Game/Materials/M_Gold.M_Gold"))
  (Variables|Default|SetCoinValue (Utilities|Select :Index _output_get :Option%200 1 :Option%201 2 :Option%202 5)))